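; AI controller that moves an NPC toward its active target actor, with jump handling for nav links.
; Nav links queue unique destinations, which Tick follows before resuming pursuit of the pawn's RefActive.
; Destinations above the tagged FeetPoint mesh trigger jumps with forward air input, and are dropped once horizontally within tolerance and not above the feet.
; FixStale is called each tick but empty; its stuck-timeout queue clearing is disconnected.
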(event EventTick
  (params (DeltaSeconds :type Float%20%28single-precision%29))
  (Utilities|FlowControl|Sequence
    (:then_0
      (if (> (Utilities|Array|Length (Variables|Default|GetDestinationLocations%20)) 0)
        (CallFunction|NavLinkNodeContinue)
        (else
          (CallFunction|MoveForward))))
    (:then_1
      (CallFunction|FixStale))))

(event EventBeginPlay)

(event Custom|Jump
  (bind _ascharacter (Utilities|Casting|CastToCharacter (Pawn|GetControlledPawn)))
  (Character|Jump _ascharacter))

(event Custom|NavLinkNode%20Initiate
  (params (Destination :type Vector))
  ;[1 1 1] Add destination if a navlink is reached
  (if (== (Utilities|Array|FindItem (Variables|Default|GetDestinationLocations%20) Destination) -1)
    (Utilities|Array|Add (Variables|Default|GetDestinationLocations%20) Destination)))

(fn ConstructionScript)

(fn NavLinkNodeContinue
  (bind _returnvalue (Pawn|GetControlledPawn))
  (bind _destinationlocations_ (Variables|Default|GetDestinationLocations%20))
  (bind _returnvalue_2 (Actor|GetComponentsbyTag _returnvalue "/Script/Engine.StaticMeshComponent" "FeetPoint"))
  (bind _output (Utilities|Array|Get(acopy) _destinationlocations_))
  (bind _output_2 (Utilities|Array|Get(acopy) _returnvalue_2))
  (bind _returnvalue_3 (Transformation|GetWorldLocation _output_2))
  (Utilities|FlowControl|Sequence
    (:then_0
      ;[1 1 1] Check if navlink destination reached (horizontal)
      (if (>= (Variables|Default|GetDestinationTolerance) (Math|Vector2D|Vector2DLength (- (Math|Vector2D|MakeVector2D (.x _output) (.y _output)) (Math|Vector2D|MakeVector2D (.x _returnvalue_3) (.y _returnvalue_3)))))
        ;[1 1 1] Check if the destionation from the navlink is higher than the current place of the character
        (if (not (> (.z (Utilities|Array|Get(acopy) (Variables|Default|GetDestinationLocations%20))) (.z (Transformation|GetWorldLocation (Utilities|Array|Get(acopy) (Actor|GetComponentsbyTag (Pawn|GetControlledPawn) "/Script/Engine.StaticMeshComponent" "FeetPoint"))))))
          ;[1 1 1] Remove the node if reached
          (Utilities|Array|RemoveIndex (Variables|Default|GetDestinationLocations%20)))))
    (:then_1
      (bind _ascharacter (Utilities|Casting|CastToCharacter (Pawn|GetControlledPawn)))
      (Utilities|FlowControl|Sequence
        (:then_0
          (if (not (AI|Components|NavMovement|IsFalling (Variables|/Script/Engine.Character|GetCharacterMovement _ascharacter)))
            ;[1 1 1] Check if the destionation from the navlink is higher than the current place of the character
            (if (> (.z (Utilities|Array|Get(acopy) (Variables|Default|GetDestinationLocations%20))) (.z (Transformation|GetWorldLocation (Utilities|Array|Get(acopy) (Actor|GetComponentsbyTag (Pawn|GetControlledPawn) "/Script/Engine.StaticMeshComponent" "FeetPoint")))))
              (CallFunction|Jump))))
        (:then_1
          (if (AI|Components|NavMovement|IsFalling (Variables|/Script/Engine.Character|GetCharacterMovement _ascharacter))
            (Pawn|Input|AddMovementInput _ascharacter (Transformation|GetActorForwardVector (Pawn|GetControlledPawn)) 1.0 false)
            (else
              (AI|Navigation|MovetoLocation (Utilities|Array|Get(acopy) (Variables|Default|GetDestinationLocations%20)) -1.0 true true false true 0))))))))

(fn MoveForward
  ;[1 1 1] Check if there are no navlink nodes to follow
  (if (<= (Utilities|Array|Length (Variables|Default|GetDestinationLocations%20)) 0)
    (bind _asbp_aicharacters (Utilities|Casting|CastToBP_AICharacters (Pawn|GetControlledPawn)))
    (if (not (AI|Components|NavMovement|IsFalling (Variables|/Script/Engine.Character|GetCharacterMovement _asbp_aicharacters)))
      (Utilities|IsValid (Variables|/Game/NPCs/BP_AICharacters.BP_AICharacters_C|GetRefActive _asbp_aicharacters)
        (:Is%20Valid
          (AI|Navigation|MovetoActor (Variables|/Game/NPCs/BP_AICharacters.BP_AICharacters_C|GetRefActive _asbp_aicharacters) 1.5e+02 false true false 0))))
    (else
      (CallFunction|NavLinkNodeContinue))))

(fn FixStale)