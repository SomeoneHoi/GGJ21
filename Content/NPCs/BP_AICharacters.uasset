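; NPC character that tracks a nearby player, offers an interact prompt and reacts to being killed.
; An overlap sphere binds that player's PC_InGame interact event, which sets Moving to hide the prompt; Tick turns the widget toward the player and scales walk speed by distance.
; Hit switches on a fixed Burn rather than its Type, so the killed NPC runs in circles until an actor hit ragdolls it.
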(event OnComponentBeginOverlap(OverlapSphere)
  (params (OverlappedComponent :type Primitive%20Component%20Object%20Reference) (OtherActor :type Actor%20Object%20Reference) (OtherComp :type Primitive%20Component%20Object%20Reference) (OtherBodyIndex :type Integer) (bFromSweep :type Boolean) (SweepResult :type Hit%20Result%20Structure%20%28by%20ref%29))
  ;[1 1 1] Set to available players around
  (bind _asbp_player (Utilities|Casting|CastToBP_Player OtherActor))
  (Utilities|Array|Add (Variables|PlayerFollow|GetReferenceOverlaps) _asbp_player)
  (Utilities|IsValid (Variables|PlayerFollow|GetRefActive)
    (:Is%20Not%20Valid
      (bind _output_get (Variables|PlayerFollow|SetRefActive _asbp_player))
      (bind _aspc_in_game (Utilities|Casting|CastToPC_InGame (Pawn|GetController _output_get)))
      (EventDispatchers|BindEventtoOnInteract _aspc_in_game (delegate Custom|OnInteract)))))

(event Custom|OnInteract
  (params (Bool :type Boolean))
  (if Bool
    (Utilities|IsValid (Variables|PlayerFollow|GetRefActive)
      (:Is%20Valid
        (Variables|PlayerFollow|SetMoving true)))))

(event Custom|On%20Hit
  (params (SelfActor :type Actor%20Object%20Reference) (OtherActor :type Actor%20Object%20Reference) (NormalImpulse :type Vector) (Hit :type Hit%20Result%20Structure%20%28by%20ref%29))
  (if (Variables|Kill|GetKilled)
    (Physics|SetSimulatePhysics (Variables|Character|GetMesh) true)))

(event EventTick
  (params (DeltaSeconds :type Float%20%28single-precision%29))
  (CallFunction|Widgets)
  (CallFunction|Movement)
  (Collision|BindEventtoOnActorHit (delegate Custom|On%20Hit)))

(event Collision|EventActorEndOverlap
  (params (OtherActor :type Actor%20Object%20Reference))
  (bind _asbp_player (Utilities|Casting|CastToBP_Player OtherActor))
  (if (== (Variables|PlayerFollow|GetRefActive) _asbp_player)
    (if (not (Variables|PlayerFollow|GetMoving))
      (Utilities|Array|RemoveItem (Variables|PlayerFollow|GetReferenceOverlaps) _asbp_player :!label _label)
      (bind _aspc_in_game (Utilities|Casting|CastToPC_InGame (Pawn|GetController _asbp_player)))
      (EventDispatchers|UnbindEventfromOnInteract _aspc_in_game (delegate Custom|OnInteract))
      (Variables|PlayerFollow|SetRefActive 0))
    (else
      (goto _label))))

(fn ConstructionScript)

(fn Widgets
  ;[1 1 1] Widgets
  (Utilities|IsValid (Variables|PlayerFollow|GetRefActive)
    (:Is%20Valid
      (if (Variables|PlayerFollow|GetMoving)
        (Development|SetHiddeninGame (Variables|Default|GetWidget) true false)
        (Development|SetHiddeninGame (Variables|Default|GetStaticMesh) true false)
        (else
          (Development|SetHiddeninGame (Variables|Default|GetWidget) false false)
          (Transformation|SetWorldRotation (Variables|Default|GetWidget) (Math|Rotator|FindLookatRotation (Transformation|GetActorLocation) (Transformation|GetActorLocation (Variables|PlayerFollow|GetRefActive))) false false))))
    (:Is%20Not%20Valid
      (Development|SetHiddeninGame (Variables|Default|GetWidget) true false))))

(fn Movement
  (Utilities|FlowControl|Sequence
    (:then_0
      (Utilities|IsValid (Variables|PlayerFollow|GetRefActive)
        (:Is%20Valid
          (Variables|/Script/Engine.CharacterMovementComponent|SetMaxWalkSpeed (Variables|Character|GetCharacterMovement) (Math|Float|Clamp(Float) (* (/ (Math|Vector|VectorLength (- (Transformation|GetActorLocation) (Transformation|GetWorldLocation (Variables|/Script/Engine.Character|GetMesh (Variables|PlayerFollow|GetRefActive))))) (Variables|PlayerFollow|GetRange)) (Variables|Movement|GetMaxWalkSpeed)) (Variables|Movement|GetMinWalkSpeed) (Variables|Movement|GetMaxWalkSpeed))))))
    (:then_1
      (if (and (Variables|Kill|GetKilled) (not (Physics|IsSimulatingPhysics (Variables|Character|GetMesh) "None")))
        (AI|Navigation|SimpleMovetoLocation (Pawn|GetController) (+ (Variables|Kill|GetKillLocation) (Math|Vector|MakeVector (+ (.x (Variables|Kill|GetKillLocation)) (* (Variables|Kill|GetRadiusMovementCircle) (Math|Trig|Cos(Degrees) (Variables|Kill|GetAngleMovementCircle)))) (+ (.y (Variables|Kill|GetKillLocation)) (* (Variables|Kill|GetRadiusMovementCircle) (Math|Trig|Sin(Degrees) (Variables|Kill|GetAngleMovementCircle)))) 0.0)))
        (bind _output_get (Variables|Kill|SetAngleMovementCircle (+ (Variables|Kill|GetAngleMovementCircle) 1.0)))
        (if (>= _output_get 3.6e+02)
          (Variables|Kill|SetAngleMovementCircle 0.0))))))

(fn Kill
  (Actor|DestroyActor))

(fn Hit
  (params (Type :type EKillType%20Enum :default "NewEnumerator0"))
  (Variables|Kill|SetKilled true)
  (switch Utilities|FlowControl|Switch|SwitchonEKillType "NewEnumerator0"
    (:NewEnumerator0
      (Variables|Kill|SetKillLocation (Transformation|GetActorLocation)))
    (:NewEnumerator1
      (Physics|SetSimulatePhysics (Variables|Character|GetMesh) true :!label _label))
    (:NewEnumerator2
      (goto _label))
    (:NewEnumerator3
      (goto _label))))