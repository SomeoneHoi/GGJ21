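; Staged in-world tutorial actor that walks the player through trap activation and follower command prompts.
; Each BP_Player overlap with its trigger advances a boolean-gated sequence, swapping prompt visibility and moving the root to the referenced AI, then the Trap.
; Short delays precede some flag changes between stages.
; An overlap after the final "move follower here" prompt destroys the actor.
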(event OnComponentBeginOverlap(Trigger)
  (params (OverlappedComponent :type Primitive%20Component%20Object%20Reference) (OtherActor :type Actor%20Object%20Reference) (OtherComp :type Primitive%20Component%20Object%20Reference) (OtherBodyIndex :type Integer) (bFromSweep :type Boolean) (SweepResult :type Hit%20Result%20Structure%20%28by%20ref%29))
  (Utilities|Casting|CastToBP_Player OtherActor)
  (if (Variables|Default|GetFirstTutorial)
    (Utilities|FlowControl|DoOnce false
      (:Completed
        (CallFunction|TutorialPart2)
        (Utilities|FlowControl|Delay 0.2)
        (Variables|Default|SetFirstTutorial false)))
    (else
      (CallFunction|TutorialPart3))))

(event Custom|Tutorial%20part%202
  (bind _defaultsceneroot (Variables|Default|GetDefaultSceneRoot))
  (bind _ai (Variables|Default|GetAI))
  (Rendering|SetVisibility (Variables|Default|GetPress%20F%20%28Activate%20trap%29) false false)
  (Transformation|SetWorldLocation _defaultsceneroot (Transformation|GetActorLocation (Utilities|ResolveSoftReference _ai)) false false)
  (Transformation|SetWorldRotation _defaultsceneroot (Transformation|GetActorRotation (Utilities|ResolveSoftReference _ai)) false false)
  (Rendering|SetVisibility (Variables|Default|GetPress%20F%20%28Follow%29) true false)
  (Variables|Default|SetSecondTutorial true))

(event Custom|Tutorial%20part%203
  (bind _trap (Variables|Default|GetTrap))
  (bind _defaultsceneroot (Variables|Default|GetDefaultSceneRoot))
  (if (Variables|Default|GetSecondTutorial)
    (Rendering|SetVisibility (Variables|Default|GetPress%20F%20%28Follow%29) false false)
    (Rendering|SetVisibility (Variables|Default|GetMove%20follower%20here) true false)
    (Transformation|SetWorldLocation _defaultsceneroot (Transformation|GetActorLocation _trap) false false)
    (Transformation|SetWorldRotation _defaultsceneroot (Transformation|GetActorRotation _trap) false false)
    (Utilities|FlowControl|Delay 0.2)
    (Variables|Default|SetSecondTutorial false)
    (Variables|Default|SetThirdTutorial true)
    (else
      (CallFunction|TutorialEnd))))

(event Custom|Tutorial%20end
  (if (Variables|Default|GetThirdTutorial)
    (Actor|DestroyActor)))

(event EventBeginPlay)

(event Collision|EventActorBeginOverlap
  (params (OtherActor :type Actor%20Object%20Reference)))

(event EventTick
  (params (DeltaSeconds :type Float%20%28single-precision%29)))

(fn ConstructionScript)