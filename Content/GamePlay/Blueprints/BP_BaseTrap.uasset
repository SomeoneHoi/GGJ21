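; Base class for one-charge traps, meant to be subclassed, that deal delayed damage by damage type.
; Overlapping TrapOverlapShape triggers an armed trap, while DamageOverlapShape tracks affected actors and can also start the Tick-driven countdown once triggered.
; On expiry, DealDamage switches on DamageType to apply plain, point or radial damage (electrical, fire and water also set Burning), then disarms.
; Functions also arm, disarm, or fully disable and re-enable the trap.
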(event OnComponentBeginOverlap(DamageOverlapShape)
  (params (OverlappedComponent :type Primitive%20Component%20Object%20Reference) (OtherActor :type Actor%20Object%20Reference) (OtherComp :type Primitive%20Component%20Object%20Reference) (OtherBodyIndex :type Integer) (bFromSweep :type Boolean) (SweepResult :type Hit%20Result%20Structure%20%28by%20ref%29))
  (if (Variables|TrapVariables|All|GetTrapExists)
    (Utilities|Array|AddUnique (Variables|TrapVariables|Timers|GetAffectedActors) OtherActor)
    (if (Variables|TrapVariables|All|GetArmed)
      (if (Variables|TrapVariables|All|GetTriggered)
        (CallFunction|StartDamageCountDown SweepResult)))))

(event OnComponentEndOverlap(DamageOverlapShape)
  (params (OverlappedComponent :type Primitive%20Component%20Object%20Reference) (OtherActor :type Actor%20Object%20Reference) (OtherComp :type Primitive%20Component%20Object%20Reference) (OtherBodyIndex :type Integer))
  (Utilities|Array|RemoveItem (Variables|TrapVariables|Timers|GetAffectedActors) OtherActor))

(event OnComponentBeginOverlap(TrapOverlapShape)
  (params (OverlappedComponent :type Primitive%20Component%20Object%20Reference) (OtherActor :type Actor%20Object%20Reference) (OtherComp :type Primitive%20Component%20Object%20Reference) (OtherBodyIndex :type Integer) (bFromSweep :type Boolean) (SweepResult :type Hit%20Result%20Structure%20%28by%20ref%29))
  ;[1 1 1] Enter trap
  (if (Variables|TrapVariables|All|GetTrapExists)
    (bind _asbp_player (Utilities|Casting|CastToBP_Player OtherActor)
      (:then
        _)
      (:CastFailed
        _))
    (Development|PrintString (Utilities|String|Append (Utilities|GetDisplayName self) "Trap area entered"))
    (if (not (== (Variables|TrapVariables|All|GetDamageType) "/Game/GamePlay/Blueprints/DamageTypes/BP_Base_DamageType.BP_Base_DamageType_C"))
      (bind _traptriggeredsuccesfully (CallFunction|TriggerTrap))
      (Development|PrintString (Utilities|String|Append (Utilities|GetDisplayName self) (Utilities|String|SelectString "Triggered succesfully " "Not armed / Not active" _traptriggeredsuccesfully) "at location: " (Utilities|String|ToString(Vector) (Transformation|GetActorLocation))) true true "(R=1.000000,G=1.000000,B=0.000000,A=1.000000)")
      (if _traptriggeredsuccesfully
        (Utilities|Casting|CastToBP_Player OtherActor)
        ;[1 1 1] Know which player triggered the trap
        (Variables|Default|SetPlayer (Utilities|ResolveSoftReference _asbp_player))
        (if (Variables|TrapVariables|All|GetStartDamageOnTrigger)
          (CallFunction|StartDamageCountDown SweepResult)))
      (else
        (Development|PrintString (Utilities|String|Append "Warning, no damage type set for " (Utilities|GetDisplayName self) "at location: " (Utilities|String|ToString(Vector) (Transformation|GetActorLocation))) true true "(R=1.000000,G=0.000000,B=0.000000,A=1.000000)")))))

(event OnComponentEndOverlap(TrapOverlapShape)
  (params (OverlappedComponent :type Primitive%20Component%20Object%20Reference) (OtherActor :type Actor%20Object%20Reference) (OtherComp :type Primitive%20Component%20Object%20Reference) (OtherBodyIndex :type Integer))
  ;[1 1 1] Exit trap
  (if (Variables|TrapVariables|All|GetTrapExists)
    (Development|PrintString (Utilities|String|Append (Utilities|GetDisplayName self) "Trap area left"))))

(event EventBeginPlay
  (bind _self self)
  (bind _damagetype (Variables|TrapVariables|All|GetDamageType))
  ;[1 1 1] Initial damage type check
  (if (Utilities|IsValidClass _damagetype)
    (bind _returnvalue (Game|ConstructObjectfromClass _damagetype self))
    (Variables|TrapVariables|All|SetDamageTypeRef _returnvalue)
    (else
      (Development|PrintString (Utilities|String|Append "No damage type set in: " (Utilities|GetDisplayName _self) "at location: " (Utilities|String|ToString(Vector) (Transformation|GetActorLocation _self))) true true "(R=1.000000,G=0.000000,B=0.000000,A=1.000000)" 1e+01))))

(event Collision|EventActorBeginOverlap
  (params (OtherActor :type Actor%20Object%20Reference))
  ;[1 0 0] Do not use this base class for traps!
  ;;[1 0.25 0] Create a child of the class instead
)

(event EventTick
  (params (DeltaSeconds :type Float%20%28single-precision%29))
  ;[1 0 0] Do not use this base class for traps!
  ;;[1 0.25 0] Create a child of the class instead
  (if (Variables|TrapVariables|Timers|GetDamageCountDownActive)
    (bind _output_get (Variables|TrapVariables|Timers|SetCurrentDamageDelayTimer (- (Variables|TrapVariables|Timers|GetCurrentDamageDelayTimer) (Utilities|Time|GetWorldDeltaSeconds))))
    (if (<= _output_get 0.0)
      (Variables|TrapVariables|Timers|SetDamageCountDownActive false)
      (CallFunction|DealDamage (Variables|TrapVariables|Timers|GetLastHitResult)))))

(fn ConstructionScript)

(fn ElectricalDamage
  (params (TrapTarget :type Actor%20Object%20Reference) (HitResult :type Hit%20Result%20Structure))
  (bind _returnvalue (Actor|GetComponentbyClass TrapTarget "/Game/Characters/Blueprints/BP_Actor_Damage_Component.BP_Actor_Damage_Component_C"))
  ;[1 1 1] Shocked in place, set on fire
  (Game|Damage|ApplyDamage TrapTarget (Variables|TrapVariables|All|GetBaseDamage) 0 self (Variables|TrapVariables|All|GetDamageType))
  (Utilities|IsValid _returnvalue
    (:Is%20Valid
      (Variables|/Game/Characters/Blueprints/BP_Actor_Damage_Component.BP_Actor_Damage_Component_C|SetBurning _returnvalue true)
      (Variables|/Game/Characters/Blueprints/BP_Actor_Damage_Component.BP_Actor_Damage_Component_C|SetBurnTimeRemaining _returnvalue (Variables|TrapVariables|All|GetBurnTimer))
      (return))
    (:Is%20Not%20Valid
      (Development|PrintString (Utilities|String|Append "Warning, no BP_ActorDamageComponent set on: " (Utilities|GetDisplayName TrapTarget))))))

(fn LocalizedDamage
  (params (TrapTarget :type Actor%20Object%20Reference) (HitResult :type Hit%20Result%20Structure))
  ;[1 1 1] Destroyed in place
  (Game|Damage|ApplyDamage TrapTarget (Variables|TrapVariables|All|GetBaseDamage) 0 self (Variables|TrapVariables|All|GetDamageType))
  (return))

(fn BluntForceDamage(Point)
  (params (TrapTarget :type Actor%20Object%20Reference) (Hit%20Result :type Hit%20Result%20Structure))
  ;[1 1 1] Knocked away
  (Game|Damage|ApplyPointDamage TrapTarget (Variables|TrapVariables|All|GetBaseDamage) (- (.Location (Collision|BreakHitResult Hit%20Result)) (Transformation|GetActorLocation)) Hit%20Result 0 0 (Variables|TrapVariables|All|GetDamageType))
  (return))

(fn ExplosiveDamage(RadiusFallOff)
  (params (TrapTarget :type Actor%20Object%20Reference) (HitResult :type Hit%20Result%20Structure))
  ;[1 1 1] Explodes / flies away
  (Class|GameplayStatics|ApplyRadialDamagewithFalloff (Variables|TrapVariables|All|GetBaseDamage) (Variables|TrapVariables|Radial|WithFallOff|GetMinimumDamage) (Transformation|GetActorLocation) (Variables|TrapVariables|Radial|WithFallOff|GetDamageInnerRadius) (.SphereRadius (Collision|GetComponentBounds (Variables|Default|GetDamageOverlapShape))) (Variables|/Script/Engine.DamageType|GetDamageFalloff (Variables|TrapVariables|All|GetDamageTypeRef)) (Variables|TrapVariables|All|GetDamageType) (Variables|TrapVariables|Radial|All|GetIgnoreActors) self 0 (Variables|TrapVariables|Radial|All|GetDamagePreventionChannel))
  (return))

(fn FireDamage
  (params (TrapTarget :type Actor%20Object%20Reference) (Hit%20Result :type Hit%20Result%20Structure))
  (bind _returnvalue (Actor|GetComponentbyClass TrapTarget "/Game/Characters/Blueprints/BP_Actor_Damage_Component.BP_Actor_Damage_Component_C"))
  ;[1 1 1] Burns
  (Game|Damage|ApplyDamage TrapTarget (Variables|TrapVariables|All|GetBaseDamage) 0 self (Variables|TrapVariables|All|GetDamageType))
  (Utilities|IsValid _returnvalue
    (:Is%20Valid
      (Variables|/Game/Characters/Blueprints/BP_Actor_Damage_Component.BP_Actor_Damage_Component_C|SetBurning _returnvalue true)
      (Variables|/Game/Characters/Blueprints/BP_Actor_Damage_Component.BP_Actor_Damage_Component_C|SetBurnTimeRemaining _returnvalue (Variables|TrapVariables|All|GetBurnTimer))
      (return))
    (:Is%20Not%20Valid
      (Development|PrintString (Utilities|String|Append "Warning, no BP_ActorDamageComponent set on: " (Utilities|GetDisplayName TrapTarget))))))

(fn WaterDamage
  (params (TrapTarget :type Actor%20Object%20Reference) (Hit%20Result :type Hit%20Result%20Structure))
  (bind _returnvalue (Actor|GetComponentbyClass TrapTarget "/Game/Characters/Blueprints/BP_Actor_Damage_Component.BP_Actor_Damage_Component_C"))
  ;[1 1 1] Drawning
  (Game|Damage|ApplyDamage TrapTarget (Variables|TrapVariables|All|GetBaseDamage) 0 self (Variables|TrapVariables|All|GetDamageType))
  (Utilities|IsValid _returnvalue
    (:Is%20Valid
      (Variables|/Game/Characters/Blueprints/BP_Actor_Damage_Component.BP_Actor_Damage_Component_C|SetBurning _returnvalue true)
      (Variables|/Game/Characters/Blueprints/BP_Actor_Damage_Component.BP_Actor_Damage_Component_C|SetBurnTimeRemaining _returnvalue (Variables|TrapVariables|All|GetBurnTimer))
      (return))
    (:Is%20Not%20Valid
      (Development|PrintString (Utilities|String|Append "Warning, no BP_ActorDamageComponent set on: " (Utilities|GetDisplayName TrapTarget))))))

(fn TriggerTrap
  (if (Variables|TrapVariables|All|GetTrapExists)
    ;[1 1 0] Only one charge per trap atm
    (if (Variables|TrapVariables|All|GetArmed)
      (Variables|TrapVariables|All|SetTriggered true)
      (return true)
      (else
        (return false)))
    (else
      (return false))))

(fn DealDamage
  (params (HitResult :type Hit%20Result%20Structure))
  (if (Variables|TrapVariables|All|GetTrapExists)
    ;[1 1 1] All actors still inside the DamageShape
    (for _array_element (Variables|TrapVariables|Timers|GetAffectedActors)
      (Utilities|SwitchonDamageType (Variables|TrapVariables|All|GetDamageType)
        (:Default%28Shouldn't?%29
          (Development|PrintString (Utilities|String|Append "Warning, no damage type set for " (Utilities|GetDisplayName self) "at location: " (Utilities|String|ToString(Vector) (Transformation|GetActorLocation))) true true "(R=1.000000,G=0.000000,B=0.000000,A=1.000000)"))
        (:BluntForceDamage
          (DamageTypes|BluntForceDamage(Point) _array_element HitResult))
        (:ElectricalDamage
          (DamageTypes|ElectricalDamage _array_element HitResult))
        (:ExplosiveDamage
          (DamageTypes|ExplosiveDamage(RadiusFallOff) _array_element HitResult))
        (:FireDamage
          (DamageTypes|FireDamage _array_element HitResult))
        (:LocalizedDamage
          (DamageTypes|LocalizedDamage _array_element HitResult))
        (:WaterDamage
          (DamageTypes|WaterDamage _array_element HitResult))))
    (Variables|TrapVariables|All|SetTriggered false)
    (bind _output_get (Variables|TrapVariables|All|SetArmed false))
    (return true _output_get)
    (else
      (return false (Variables|TrapVariables|All|GetArmed)))))

(fn ArmTrap
  (Development|PrintString (Utilities|String|Append "Armed: " (Utilities|GetDisplayName self)))
  (Variables|TrapVariables|All|SetArmed true)
  (return))

(fn DisarmTrap
  (Development|PrintString (Utilities|String|Append "Disarmed: " (Utilities|GetDisplayName self)))
  (Variables|TrapVariables|All|SetArmed false)
  (return))

(fn DisableTrapCompletely
  (Variables|TrapVariables|All|SetTrapExists false)
  (Rendering|SetActorHiddenInGame true)
  (return))

(fn ReEnableTrapCompletely
  (Variables|TrapVariables|All|SetTrapExists true)
  (Rendering|SetActorHiddenInGame false)
  (return))

(fn StartDamageCountDown
  (params (LastHitResult :type Hit%20Result%20Structure))
  (if (Variables|TrapVariables|Timers|GetDamageCountDownActive)
    (return)
    (else
      (Variables|TrapVariables|Timers|SetLastHitResult LastHitResult)
      (Variables|TrapVariables|Timers|SetDamageCountDownActive true)
      (Variables|TrapVariables|Timers|SetCurrentDamageDelayTimer (Variables|TrapVariables|Timers|GetTrapDamageDelayTimer))
      (return))))