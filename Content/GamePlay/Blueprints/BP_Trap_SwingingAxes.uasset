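; Swinging axe trap Blueprint, a child of a parent trap class that animates an axe through the arm, trigger and disarm states.
; On BeginPlay it attaches DamageOverlapShape to the Axe's DamageSocket, keeping world transform, so the shape follows the animation.
; Arming plays a one-shot swing start animation, a successful parent trigger starts the looping swing, and disarming stops it.
; Overlap handling is deferred to the parent.
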(event EventBeginPlay
  (|CallParentFunction)
  (Transformation|AttachComponentToComponent (Variables|Default|GetDamageOverlapShape) (Variables|Default|GetAxe) "DamageSocket" "KeepWorld" "KeepWorld" "KeepWorld" true))

(event Collision|EventActorBeginOverlap
  (params (OtherActor :type Actor%20Object%20Reference))
  (|CallParentFunction OtherActor))

(event EventTick
  (params (DeltaSeconds :type Float%20%28single-precision%29))
  (|CallParentFunction DeltaSeconds) ; This node is disabled and will not be called.\nDrag off pins to build functionality.
)

(fn ConstructionScript
  (|CallParentFunction))

(fn ArmTrap
  (Components|Animation|PlayAnimation (Variables|Default|GetAxe) "/Game/Art/Models/AxeSwingStart_Anim.AxeSwingStart_Anim" false)
  (|CallParentFunction))

(fn TriggerTrap
  (bind _traptriggeredsuccesfully (|CallParentFunction))
  (if _traptriggeredsuccesfully
    (Components|Animation|PlayAnimation (Variables|Default|GetAxe) "/Game/Art/Models/AxeSwingLoop_Anim.AxeSwingLoop_Anim" true))
  (return _traptriggeredsuccesfully))

(fn DisarmTrap
  (|CallParentFunction)
  (Audio|Components|Audio|Stop (Variables|Default|GetAxe))
  (return))