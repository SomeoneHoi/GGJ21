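; BP_Trap is a base trap actor that deals damage to a target when TriggerTrap fires, one shot per load until ResetTrap reloads it.
; A macro switches on the DamageType class to route hits to point damage for blunt force, radial falloff for explosive, or plain damage for fire and water.
; BeginPlay prints a red warning if no damage type is set, and DisableTrap is a placeholder that only unloads it.
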(event Custom|TriggerTrap
  (params (TrapTarget :type Actor%20Object%20Reference) (HitResult :type Hit%20Result%20Structure))
  (bind _damagetype (Variables|TrapVariables|All|GetDamageType))
  (if (Utilities|IsValidClass _damagetype)
    ;[1 1 0] Only one load per trap atm
    (if (Variables|TrapVariables|All|GetLoaded)
      (Variables|TrapVariables|All|SetLoaded false)
      (Utilities|SwitchonDamageType _damagetype
        (:BluntForceDamage
          (DamageTypes|BluntForceDamage(Point) TrapTarget HitResult))
        (:ExplosiveDamage
          (DamageTypes|ExplosiveDamage(RadiusFallOff) TrapTarget HitResult))
        (:FireDamage
          (DamageTypes|FireDamage TrapTarget HitResult))
        (:WaterDamage
          (DamageTypes|WaterDamage TrapTarget HitResult))))))

(event Custom|ResetTrap
  (Variables|TrapVariables|All|SetLoaded true))

(event Custom|DisableTrap
  ;[1 1 0] Todo: Write actual disable
  (Variables|TrapVariables|All|SetLoaded false))

(event EventBeginPlay
  (bind _self self)
  (if (not (Utilities|IsValidClass (Variables|TrapVariables|All|GetDamageType)))
    (Development|PrintString (Utilities|String|Append "No damage type set in: " (Utilities|GetDisplayName _self) "at location: " (Utilities|String|ToString(Vector) (Transformation|GetActorLocation _self))) true true "(R=1.000000,G=0.000000,B=0.000000,A=1.000000)" 1e+01)))

(event Collision|EventActorBeginOverlap
  (params (OtherActor :type Actor%20Object%20Reference))
  ;[1 0 0] Do not use this base class for traps!
)

(event EventTick
  (params (DeltaSeconds :type Float%20%28single-precision%29))
  ;[1 0 0] Do not use this base class for traps!
)

(fn ConstructionScript)

(fn BluntForceDamage(Point)
  (params (TrapTarget :type Actor%20Object%20Reference) (Hit%20Result :type Hit%20Result%20Structure))
  (Game|Damage|ApplyPointDamage TrapTarget (Variables|TrapVariables|All|GetBaseDamage) (- (.Location (Collision|BreakHitResult Hit%20Result)) (Transformation|GetActorLocation)) Hit%20Result 0 0 (Variables|TrapVariables|All|GetDamageType))
  (return))

(fn ExplosiveDamage(RadiusFallOff)
  (params (TrapTarget :type Actor%20Object%20Reference) (HitResult :type Hit%20Result%20Structure))
  (Class|GameplayStatics|ApplyRadialDamagewithFalloff (Variables|TrapVariables|All|GetBaseDamage) (Variables|TrapVariables|Radial|WithFallOff|GetMinimumDamage) (Variables|TrapVariables|Radial|All|GetOrigin) (Variables|TrapVariables|Radial|WithFallOff|GetDamageInnerRadius) (Variables|TrapVariables|Radial|WithFallOff|GetDamageOuterRadius) (Variables|TrapVariables|Radial|WithFallOff|GetDamageFallOff) (Variables|TrapVariables|All|GetDamageType) (Variables|TrapVariables|Radial|All|GetIgnoreActors) self 0 (Variables|TrapVariables|Radial|All|GetDamagePreventionChannel)))

(fn FireDamage
  (params (TrapTarget :type Actor%20Object%20Reference) (Hit%20Result :type Hit%20Result%20Structure))
  (Game|Damage|ApplyDamage TrapTarget (Variables|TrapVariables|All|GetBaseDamage) 0 self (Variables|TrapVariables|All|GetDamageType))
  (return))

(fn WaterDamage
  (params (TrapTarget :type Actor%20Object%20Reference) (Hit%20Result :type Hit%20Result%20Structure))
  (Game|Damage|ApplyDamage TrapTarget (Variables|TrapVariables|All|GetBaseDamage) 0 self (Variables|TrapVariables|All|GetDamageType))
  (return))