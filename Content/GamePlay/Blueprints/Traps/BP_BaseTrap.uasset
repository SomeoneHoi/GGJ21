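; Base trap Blueprint, meant for subclassing, with an arm, trigger, damage, disarm, disable and re-enable cycle.
; The current state lives in a Blackboard enum, changed through SetNewState with optional transition safety checks, alongside reset/tick timer helpers per phase.
; Separate trigger and damage overlap shapes track actors and request state changes.
; DealDamage switches on DamageType class to apply plain, point or radial damage, with burning for fire, electrical and water.
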(event OnComponentBeginOverlap(DamageOverlapShape)
  (params (OverlappedComponent :type Primitive%20Component%20Object%20Reference) (OtherActor :type Actor%20Object%20Reference) (OtherComp :type Primitive%20Component%20Object%20Reference) (OtherBodyIndex :type Integer) (bFromSweep :type Boolean) (SweepResult :type Hit%20Result%20Structure%20%28by%20ref%29))
  (Utilities|Array|AddUnique (Variables|BehaviourTree|Damage|GetDamagedActors) OtherActor)
  (bind _currentstate (BehaviourTree|State|GetCurrentState))
  (if (Utilities|Enum|Equal(Enum) _currentstate "NewEnumerator14")
    (BehaviourTree|State|SetNewState "NewEnumerator4" false)))

(event OnComponentEndOverlap(DamageOverlapShape)
  (params (OverlappedComponent :type Primitive%20Component%20Object%20Reference) (OtherActor :type Actor%20Object%20Reference) (OtherComp :type Primitive%20Component%20Object%20Reference) (OtherBodyIndex :type Integer))
  (Utilities|Array|RemoveItem (Variables|BehaviourTree|Damage|GetDamagedActors) OtherActor))

(event OnComponentBeginOverlap(TrapOverlapShape)
  (params (OverlappedComponent :type Primitive%20Component%20Object%20Reference) (OtherActor :type Actor%20Object%20Reference) (OtherComp :type Primitive%20Component%20Object%20Reference) (OtherBodyIndex :type Integer) (bFromSweep :type Boolean) (SweepResult :type Hit%20Result%20Structure%20%28by%20ref%29))
  ;[1 1 1] Enter trap
  (Utilities|Array|AddUnique (Variables|BehaviourTree|Trigger|GetTriggeredActors) 0)
  (Debug|PrintString|DebugStringTrapAreaEntered)
  (bind _currentstate (BehaviourTree|State|GetCurrentState))
  (if (Utilities|Enum|Equal(Enum) _currentstate "NewEnumerator13")
    (BehaviourTree|State|SetNewState "NewEnumerator5" false)))

(event OnComponentEndOverlap(TrapOverlapShape)
  (params (OverlappedComponent :type Primitive%20Component%20Object%20Reference) (OtherActor :type Actor%20Object%20Reference) (OtherComp :type Primitive%20Component%20Object%20Reference) (OtherBodyIndex :type Integer))
  ;[1 1 1] Exit trap
  (Utilities|Array|RemoveItem (Variables|BehaviourTree|Trigger|GetTriggeredActors) 0)
  (Debug|PrintString|DebugStringTrapAreaLeft))

(event EventBeginPlay
  (bind _damagetype (Variables|TrapVariables|GetDamageType))
  ;[1 1 1] Initial damage type check
  (if (Utilities|IsValidClass _damagetype)
    (bind _returnvalue (Game|ConstructObjectfromClass _damagetype self))
    (Variables|TrapVariables|SetDamageTypeRef _returnvalue)
    (BehaviourTree|Init|InitializeTimers)
    ;[1 1 1] Can be done through state selection itself, boolean is designer friendlier with previous implementation?
    (if (Variables|TrapVariables|GetArmed)
      (BehaviourTree|State|SetNewState "NewEnumerator1" true))
    (else
      (Debug|PrintString|DebugStringWarningNoDamageType))))

(event Collision|EventActorBeginOverlap
  (params (OtherActor :type Actor%20Object%20Reference))
  ;[1 0 0] Do not use this base class for traps!
  ;;[1 0.25 0] Create a child of the class instead
)

(event EventTick
  (params (DeltaSeconds :type Float%20%28single-precision%29))
  ;[1 0 0] Do not use this base class for traps!
  ;;[1 0.25 0] Create a child of the class instead
)

(fn ConstructionScript)

(fn ElectricalDamage
  (params (TrapTarget :type Actor%20Object%20Reference) (HitResult :type Hit%20Result%20Structure))
  (bind _returnvalue (Actor|GetComponentbyClass TrapTarget "/Game/Characters/Blueprints/BP_Actor_Damage_Component.BP_Actor_Damage_Component_C"))
  ;[1 1 1] Shocked in place, set on fire
  (Game|Damage|ApplyDamage TrapTarget (Variables|TrapVariables|GetBaseDamage) 0 self (Variables|TrapVariables|GetDamageType))
  (Utilities|IsValid _returnvalue
    (:Is%20Valid
      (Variables|/Game/Characters/Blueprints/BP_Actor_Damage_Component.BP_Actor_Damage_Component_C|SetBurning _returnvalue true)
      (Variables|/Game/Characters/Blueprints/BP_Actor_Damage_Component.BP_Actor_Damage_Component_C|SetBurnTimeRemaining _returnvalue (Variables|TrapVariables|GetBurnTimer))
      (return))
    (:Is%20Not%20Valid
      (Development|PrintString (Utilities|String|Append "Warning, no BP_ActorDamageComponent set on: " (Utilities|GetDisplayName TrapTarget))))))

(fn LocalizedDamage
  (params (TrapTarget :type Actor%20Object%20Reference) (HitResult :type Hit%20Result%20Structure))
  ;[1 1 1] Destroyed in place
  (Game|Damage|ApplyDamage TrapTarget (Variables|TrapVariables|GetBaseDamage) 0 self (Variables|TrapVariables|GetDamageType))
  (return))

(fn BluntForceDamage(Point)
  (params (TrapTarget :type Actor%20Object%20Reference) (Hit%20Result :type Hit%20Result%20Structure))
  ;[1 1 1] Knocked away
  (Game|Damage|ApplyPointDamage TrapTarget (Variables|TrapVariables|GetBaseDamage) (- (.Location (Collision|BreakHitResult Hit%20Result)) (Transformation|GetActorLocation)) Hit%20Result 0 self (Variables|TrapVariables|GetDamageType))
  (return))

(fn ExplosiveDamage(RadiusFallOff)
  (params (TrapTarget :type Actor%20Object%20Reference) (HitResult :type Hit%20Result%20Structure))
  ;[1 1 1] Explodes / flies away
  (Class|GameplayStatics|ApplyRadialDamagewithFalloff (Variables|TrapVariables|GetBaseDamage) (Variables|TrapVariables|GetMinimumDamage) (Transformation|GetActorLocation) (Variables|TrapVariables|GetDamageInnerRadius) (.SphereRadius (Collision|GetComponentBounds (Variables|Default|GetDamageOverlapShape))) (Variables|/Script/Engine.DamageType|GetDamageFalloff (Variables|TrapVariables|GetDamageTypeRef)) (Variables|TrapVariables|GetDamageType) (Variables|TrapVariables|GetIgnoreActors) self 0 (Variables|TrapVariables|GetDamagePreventionChannel))
  (return))

(fn FireDamage
  (params (TrapTarget :type Actor%20Object%20Reference) (Hit%20Result :type Hit%20Result%20Structure))
  (bind _returnvalue (Actor|GetComponentbyClass TrapTarget "/Game/Characters/Blueprints/BP_Actor_Damage_Component.BP_Actor_Damage_Component_C"))
  ;[1 1 1] Burns
  (Game|Damage|ApplyDamage TrapTarget (Variables|TrapVariables|GetBaseDamage) 0 self (Variables|TrapVariables|GetDamageType))
  (Utilities|IsValid _returnvalue
    (:Is%20Valid
      (Variables|/Game/Characters/Blueprints/BP_Actor_Damage_Component.BP_Actor_Damage_Component_C|SetBurning _returnvalue true)
      (Variables|/Game/Characters/Blueprints/BP_Actor_Damage_Component.BP_Actor_Damage_Component_C|SetBurnTimeRemaining _returnvalue (Variables|TrapVariables|GetBurnTimer))
      (return))
    (:Is%20Not%20Valid
      (Development|PrintString (Utilities|String|Append "Warning, no BP_ActorDamageComponent set on: " (Utilities|GetDisplayName TrapTarget))))))

(fn WaterDamage
  (params (TrapTarget :type Actor%20Object%20Reference) (Hit%20Result :type Hit%20Result%20Structure))
  (bind _returnvalue (Actor|GetComponentbyClass TrapTarget "/Game/Characters/Blueprints/BP_Actor_Damage_Component.BP_Actor_Damage_Component_C"))
  ;[1 1 1] Drawning
  (Game|Damage|ApplyDamage TrapTarget (Variables|TrapVariables|GetBaseDamage) 0 self (Variables|TrapVariables|GetDamageType))
  (Utilities|IsValid _returnvalue
    (:Is%20Valid
      (Variables|/Game/Characters/Blueprints/BP_Actor_Damage_Component.BP_Actor_Damage_Component_C|SetBurning _returnvalue true)
      (Variables|/Game/Characters/Blueprints/BP_Actor_Damage_Component.BP_Actor_Damage_Component_C|SetBurnTimeRemaining _returnvalue (Variables|TrapVariables|GetBurnTimer))
      (return))
    (:Is%20Not%20Valid
      (Development|PrintString (Utilities|String|Append "Warning, no BP_ActorDamageComponent set on: " (Utilities|GetDisplayName TrapTarget))))))

(fn StartDamageCountDown
  (params (LastHitResult :type Hit%20Result%20Structure))
  (if (Variables|TrapVariables|GetDamageCountDownActive)
    (return)
    (else
      (Variables|TrapVariables|SetLastHitResult LastHitResult)
      (Variables|TrapVariables|SetDamageCountDownActive true)
      (Variables|TrapVariables|SetCurrentDamageDelayTimer (Variables|TrapVariables|GetTrapDamageDelayTimer))
      (return))))

(fn ReEnableTrapCompletely
  (Variables|TrapVariables|SetTrapExists true)
  (Variables|/Script/Engine.PrimitiveComponent|SetbGenerateOverlapEvents (Variables|Default|GetTrapOverlapShape) true)
  (Variables|/Script/Engine.PrimitiveComponent|SetbGenerateOverlapEvents (Variables|Default|GetDamageOverlapShape) true)
  (Rendering|SetActorHiddenInGame false)
  (return))

(fn ReEnableCountDownTimerReset
  (Variables|BehaviourTree|ReEnable|SetReEnableCountDownTimeCurrent (Variables|BehaviourTree|ReEnable|GetReEnableCountDownTime))
  (return))

(fn ReEnableCountDownTimerTick
  (params (DeltaTime :type Float%20%28single-precision%29))
  (bind _output_get (Variables|BehaviourTree|ReEnable|SetReEnableCountDownTimeCurrent (- (Variables|BehaviourTree|ReEnable|GetReEnableCountDownTimeCurrent) DeltaTime)))
  (if (<= _output_get 0.0)
    (return true)
    (else
      (return false))))

(fn DisableTrapCompletely
  (Variables|TrapVariables|SetTrapExists false)
  (Variables|/Script/Engine.PrimitiveComponent|SetbGenerateOverlapEvents (Variables|Default|GetTrapOverlapShape) false)
  (Variables|/Script/Engine.PrimitiveComponent|SetbGenerateOverlapEvents (Variables|Default|GetDamageOverlapShape) false)
  (Utilities|Array|Clear (Variables|BehaviourTree|Trigger|GetTriggeredActors))
  (Utilities|Array|Clear (Variables|BehaviourTree|Damage|GetDamagedActors))
  (Rendering|SetActorHiddenInGame true)
  (return))

(fn DisableCountDownTimerReset
  (Variables|BehaviourTree|Disable|SetDisableCountDownTimeCurrent (Variables|BehaviourTree|Disable|GetDisableCountDownTime))
  (return))

(fn DisableCountDownTimerTick
  (params (DeltaTime :type Float%20%28single-precision%29))
  (bind _output_get (Variables|BehaviourTree|Disable|SetDisableCountDownTimeCurrent (- (Variables|BehaviourTree|Disable|GetDisableCountDownTimeCurrent) DeltaTime)))
  (if (<= _output_get 0.0)
    (return true)
    (else
      (return false))))

(fn ArmTrap
  (Development|PrintString (Utilities|String|Append "Armed: " (Utilities|GetDisplayName self)))
  (Variables|TrapVariables|SetArmed true)
  (return))

(fn ArmCountDownTimerReset
  (Variables|BehaviourTree|Arm|SetArmCountDownTimeCurrent (Variables|BehaviourTree|Arm|GetArmCountDownTime))
  (return))

(fn ArmCountDownTimerTick
  (params (DeltaTime :type Float%20%28single-precision%29))
  (bind _output_get (Variables|BehaviourTree|Arm|SetArmCountDownTimeCurrent (- (Variables|BehaviourTree|Arm|GetArmCountDownTimeCurrent) DeltaTime)))
  (if (<= _output_get 0.0)
    (return true)
    (else
      (return false))))

(fn DisarmTrap
  (Development|PrintString (Utilities|String|Append "Disarmed: " (Utilities|GetDisplayName self)))
  (Variables|TrapVariables|SetArmed false)
  (return))

(fn DisarmCountDownTimerReset
  (Variables|BehaviourTree|Disarm|SetDisarmCountDownTimeCurrent (Variables|BehaviourTree|Disarm|GetDisarmCountDownTime))
  (return))

(fn DisarmCountDownTimerTick
  (params (DeltaTime :type Float%20%28single-precision%29))
  (bind _output_get (Variables|BehaviourTree|Disarm|SetDisarmCountDownTimeCurrent (- (Variables|BehaviourTree|Disarm|GetDisarmCountDownTimeCurrent) DeltaTime)))
  (if (<= _output_get 0.0)
    (return true)
    (else
      (return false))))

(fn CheckTriggeredActors
  ;[1 1 1] Inside Trigger box but not triggered on overlap (spawned within?)
  (for _array_element (Collision|GetOverlappingActors (Variables|Default|GetTrapOverlapShape) "/Script/Engine.Character" :!class /Script/Engine.PrimitiveComponent)
    (Utilities|Array|AddUnique (Variables|BehaviourTree|Trigger|GetTriggeredActors) _array_element))
  (return))

(fn TriggerTrap
  (if (Variables|TrapVariables|GetTrapExists)
    ;[1 1 0] Only one charge per trap atm
    (if (Variables|TrapVariables|GetArmed)
      (Variables|TrapVariables|SetTriggered true)
      (return true)
      (else
        (return false)))
    (else
      (return false))))

(fn TriggerCountDownTimerReset
  (Variables|BehaviourTree|Trigger|SetTriggerCountDownTimeCurrent (Variables|BehaviourTree|Trigger|GetTriggerCountDownTime))
  (return))

(fn TriggerCountDownTimerTick
  (params (DeltaTime :type Float%20%28single-precision%29))
  (bind _output_get (Variables|BehaviourTree|Trigger|SetTriggerCountDownTimeCurrent (- (Variables|BehaviourTree|Trigger|GetTriggerCountDownTimeCurrent) DeltaTime)))
  (if (<= _output_get 0.0)
    (return true)
    (else
      (return false))))

(fn CheckDamageActors
  ;[1 1 1] Inside Damage box but not triggered on overlap (spawned within?)
  (for _array_element (Collision|GetOverlappingActors (Variables|Default|GetDamageOverlapShape) "/Script/Engine.Character" :!class /Script/Engine.PrimitiveComponent)
    (Utilities|Array|AddUnique (Variables|BehaviourTree|Damage|GetDamagedActors) _array_element))
  (return))

(fn DealDamage
  (params (HitResult :type Hit%20Result%20Structure))
  (if (Variables|TrapVariables|GetTrapExists)
    ;[1 1 1] All actors still inside the DamageShape
    (for _array_element (Variables|BehaviourTree|Damage|GetDamagedActors)
      (Utilities|SwitchonDamageType (Variables|TrapVariables|GetDamageType)
        (:Default%28Shouldn't?%29
          (Debug|PrintString|DebugStringWarningNoDamageType self)
          (return true false))
        (:BluntForceDamage
          (DamageTypes|BluntForceDamage(Point) _array_element HitResult))
        (:ElectricalDamage
          (DamageTypes|ElectricalDamage _array_element HitResult))
        (:ExplosiveDamage
          (DamageTypes|ExplosiveDamage(RadiusFallOff) _array_element HitResult))
        (:FireDamage
          (DamageTypes|FireDamage _array_element HitResult))
        (:LocalizedDamage
          (DamageTypes|LocalizedDamage _array_element HitResult))
        (:WaterDamage
          (DamageTypes|WaterDamage _array_element HitResult))))
    (Variables|TrapVariables|SetTriggered false)
    (bind _output_get (Variables|TrapVariables|SetArmed false))
    (return true _output_get)
    (else
      (return false (Variables|TrapVariables|GetArmed)))))

(fn DamageIntervalTimerReset
  (Variables|BehaviourTree|Damage|SetDamageIntervalTimeCurrent (Variables|BehaviourTree|Damage|GetDamageIntervalTime))
  (return))

(fn DamageIntervalTimerTick
  (params (DeltaTime :type Float%20%28single-precision%29))
  (bind _output_get (Variables|BehaviourTree|Damage|SetDamageIntervalTimeCurrent (- (Variables|BehaviourTree|Damage|GetDamageIntervalTimeCurrent) DeltaTime)))
  (if (<= _output_get 0.0)
    (return true)
    (else
      (return false))))

(fn DamagePeriodTimerReset
  (Variables|BehaviourTree|Damage|SetDamagePeriodTimeCurrent (Variables|BehaviourTree|Damage|GetDamagePeriodTime))
  (return))

(fn DamagePeriodTimerTick
  (params (DeltaTime :type Float%20%28single-precision%29))
  (bind _output_get (Variables|BehaviourTree|Damage|SetDamagePeriodTimeCurrent (- (Variables|BehaviourTree|Damage|GetDamagePeriodTimeCurrent) DeltaTime)))
  (if (<= _output_get 0.0)
    (return true)
    (else
      (return false))))

(fn DamageCountDownTimerReset
  (Variables|BehaviourTree|Damage|SetDamageCountDownTimeCurrent (Variables|BehaviourTree|Damage|GetDamageCountDownTime))
  (return))

(fn DamageCountDownTimerTick
  (params (DeltaTime :type Float%20%28single-precision%29))
  (bind _output_get (Variables|BehaviourTree|Damage|SetDamageCountDownTimeCurrent (- (Variables|BehaviourTree|Damage|GetDamageCountDownTimeCurrent) DeltaTime)))
  (if (<= _output_get 0.0)
    (return true)
    (else
      (return false))))

(fn InitializeTimers
  (BehaviourTree|ReEnable|ReEnableCountDownTimerReset)
  (BehaviourTree|Disable|DisableCountDownTimerReset)
  (BehaviourTree|Arm|ArmCountDownTimerReset)
  (BehaviourTree|Disarm|DisarmCountDownTimerReset)
  (BehaviourTree|Trigger|TriggerCountDownTimerReset)
  (BehaviourTree|Damage|DamageCountDownTimerReset)
  (BehaviourTree|Damage|DamageIntervalTimerReset)
  (BehaviourTree|Damage|DamagePeriodTimerReset)
  (return))

(fn DebugStringTrapAreaEntered
  (Development|PrintString (Utilities|String|Append (Utilities|GetDisplayName self) "Trap area entered"))
  (return))

(fn DebugStringTrapAreaLeft
  (Development|PrintString (Utilities|String|Append (Utilities|GetDisplayName self) "Trap area left"))
  (return))

(fn DebugStringTrapTriggered?
  (params (TriggerResult :type Boolean))
  (Development|PrintString (Utilities|String|Append (Utilities|GetDisplayName self) (Utilities|String|SelectString "Triggered succesfully " "Not armed / Not active" TriggerResult) "at location: " (Utilities|String|ToString(Vector) (Transformation|GetActorLocation))) true true "(R=1.000000,G=1.000000,B=0.000000,A=1.000000)")
  (return))

(fn DebugStringTrapDamaged?
  (params (DamageResult :type Boolean))
  (Development|PrintString (Utilities|String|Append (Utilities|GetDisplayName self) (Utilities|String|SelectString "Applied damage " "Failed to apply damage " DamageResult) "at location: " (Utilities|String|ToString(Vector) (Transformation|GetActorLocation))) true true "(R=1.000000,G=0.150000,B=0.000000,A=1.000000)" 0.2)
  (return))

(fn DebugStringWarningNoDamageType
  (Development|PrintString (Utilities|String|Append "Warning, no damage type set for " (Utilities|GetDisplayName self) "at location: " (Utilities|String|ToString(Vector) (Transformation|GetActorLocation))) true true "(R=1.000000,G=0.000000,B=0.000000,A=1.000000)")
  (return))

(fn GetCurrentState
  ;[1 1 1] Imagine the byte to enum converter working properly in the return node...
  (switch Utilities|FlowControl|Switch|SwitchonE_CurrentTrapState (Utilities|Enum|ByteToEnumE_CurrentTrapState (Class|BlackboardComponent|GetValueasEnum (AI|GetBlackboard self) (Variables|BehaviourTree|State|GetTrapState)))
    (:NewEnumerator12
      (return "NewEnumerator12"))
    (:NewEnumerator1
      (return "NewEnumerator1"))
    (:NewEnumerator3
      (return "NewEnumerator3"))
    (:NewEnumerator13
      (return "NewEnumerator13"))
    (:NewEnumerator5
      (return "NewEnumerator5"))
    (:NewEnumerator2
      (return "NewEnumerator2"))
    (:NewEnumerator14
      (return "NewEnumerator14"))
    (:NewEnumerator4
      (return "NewEnumerator4"))
    (:NewEnumerator6
      (return "NewEnumerator6"))
    (:NewEnumerator15
      (return "NewEnumerator15"))
    (:NewEnumerator7
      (return "NewEnumerator7"))
    (:NewEnumerator0
      (return "NewEnumerator0"))
    (:NewEnumerator16
      (return "NewEnumerator16"))
    (:NewEnumerator8
      (return "NewEnumerator8"))
    (:NewEnumerator9
      (return "NewEnumerator9"))
    (:NewEnumerator17
      (return "NewEnumerator17"))
    (:NewEnumerator11
      (return "NewEnumerator11"))
    (:NewEnumerator10
      (return "NewEnumerator10"))
    (:NewEnumerator18
      (return "NewEnumerator18"))))

(fn SetNewState
  (params (NewState :type E_CurrentTrapState%20Enum :default "NewEnumerator12") (IgnoreSafety :type Boolean))
  (if IgnoreSafety
    _
    (else
      (bind _safe (BehaviourTree|State|CheckSafeStateSwitching NewState))
      (if _safe
        _
        (else
          (return false)))))
  (AI|Components|Blackboard|SetValueasEnum (AI|GetBlackboard self) (Variables|BehaviourTree|State|GetTrapState) NewState)
  (return true))

(fn CheckSafeStateSwitching
  (params (NewState :type E_CurrentTrapState%20Enum :default "NewEnumerator12"))
  ;[1 1 1] All state combinations that can break the gameplay
  (bind _currentstate (BehaviourTree|State|GetCurrentState))
  (if (Utilities|Enum|Equal(Enum) NewState "NewEnumerator12")
    _
    (elif (Utilities|Enum|Equal(Enum) NewState "NewEnumerator13")
      _
      (elif (Utilities|Enum|Equal(Enum) NewState "NewEnumerator14")
        _
        (elif (Utilities|Enum|Equal(Enum) NewState "NewEnumerator15")
          _
          (elif (Utilities|Enum|Equal(Enum) NewState "NewEnumerator16")
            _
            (elif (Utilities|Enum|Equal(Enum) NewState "NewEnumerator17")
              _
              (elif (Utilities|Enum|Equal(Enum) NewState "NewEnumerator18")
                _
                (elif (and (Math|Boolean|NANDBoolean (Utilities|Enum|NotEqual(Enum) _currentstate "NewEnumerator16") (Utilities|Enum|NotEqual(Enum) _currentstate "NewEnumerator18") (Utilities|Enum|NotEqual(Enum) _currentstate "NewEnumerator15")) (or (Utilities|Enum|Equal(Enum) NewState "NewEnumerator1") (Utilities|Enum|Equal(Enum) NewState "NewEnumerator3")))
                  (return false)
                  (elif (and (Utilities|Enum|NotEqual(Enum) _currentstate "NewEnumerator13") (or (Utilities|Enum|Equal(Enum) NewState "NewEnumerator5") (Utilities|Enum|Equal(Enum) NewState "NewEnumerator2")))
                    (return false)
                    (elif (and (Utilities|Enum|NotEqual(Enum) _currentstate "NewEnumerator14") (or (Utilities|Enum|Equal(Enum) NewState "NewEnumerator4") (Utilities|Enum|Equal(Enum) NewState "NewEnumerator6")))
                      (return false)
                      (elif (and (Utilities|Enum|NotEqual(Enum) _currentstate "NewEnumerator17") (or (Utilities|Enum|Equal(Enum) NewState "NewEnumerator11") (Utilities|Enum|Equal(Enum) NewState "NewEnumerator10")))
                        (return false)
                        (elif (and (Math|Boolean|ORBoolean (Utilities|Enum|NotEqual(Enum) _currentstate "NewEnumerator13") (Utilities|Enum|NotEqual(Enum) _currentstate "NewEnumerator14") (Utilities|Enum|NotEqual(Enum) _currentstate "NewEnumerator15") (Utilities|Enum|NotEqual(Enum) _currentstate "NewEnumerator16") (Utilities|Enum|NotEqual(Enum) _currentstate "NewEnumerator18")) (or (Utilities|Enum|Equal(Enum) NewState "NewEnumerator8") (Utilities|Enum|Equal(Enum) NewState "NewEnumerator9")))
                          (return false)
                          (elif (and (Utilities|Enum|NotEqual(Enum) _currentstate "NewEnumerator13") (or (Utilities|Enum|Equal(Enum) NewState "NewEnumerator7") (Utilities|Enum|Equal(Enum) NewState "NewEnumerator0")))
                            (return false)
                            (else
                              (return true)))))))))))))))
  (return false))