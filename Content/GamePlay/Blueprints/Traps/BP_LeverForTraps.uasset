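; BP_LeverForTraps is a lever that arms a list of linked traps when the player interacts within its trigger area.
; While the player overlaps, Tick polls the player's interact component, using a DoOnce that resets on release to fire once per press.
; Each press runs ArmTrap, which changes the Blackboard TrapState to TimeBeforeArmed only from two eligible states, then plays a flash and sound.
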(event OnComponentBeginOverlap(TriggerArea)
  (params (OverlappedComponent :type Primitive%20Component%20Object%20Reference) (OtherActor :type Actor%20Object%20Reference) (OtherComp :type Primitive%20Component%20Object%20Reference) (OtherBodyIndex :type Integer) (bFromSweep :type Boolean) (SweepResult :type Hit%20Result%20Structure%20%28by%20ref%29))
  (Utilities|Casting|CastToBP_Player OtherActor)
  (Variables|Default|SetInsideTriggerArea true)
  (Development|PrintString (Utilities|String|Append (Utilities|GetDisplayName self) "Lever area entered")))

(event OnComponentEndOverlap(TriggerArea)
  (params (OverlappedComponent :type Primitive%20Component%20Object%20Reference) (OtherActor :type Actor%20Object%20Reference) (OtherComp :type Primitive%20Component%20Object%20Reference) (OtherBodyIndex :type Integer))
  (Utilities|Casting|CastToBP_Player OtherActor)
  (Variables|Default|SetInsideTriggerArea false)
  (Development|PrintString (Utilities|String|Append (Utilities|GetDisplayName self) "Lever area left")))

(event EventBeginPlay
  (bind _returnvalue (Actor|GetActorOfClass "/Game/Characters/Blueprints/BP_Player.BP_Player_C"))
  (Utilities|IsValid (Actor|GetComponentbyClass _returnvalue "/Game/Characters/Blueprints/BP_Player_Interact_Component.BP_Player_Interact_Component_C")
    (:Is%20Valid
      (Variables|Default|SetInteractRef (Actor|GetComponentbyClass _returnvalue "/Game/Characters/Blueprints/BP_Player_Interact_Component.BP_Player_Interact_Component_C")))
    (:Is%20Not%20Valid
      (Development|PrintString "Warning: BP_Player does not have an BP_Interact_Component required for use in BP_TrapTrigger" true true "(R=1.000000,G=0.000000,B=0.000000,A=1.000000)" 1e+01))))

(event Collision|EventActorBeginOverlap
  (params (OtherActor :type Actor%20Object%20Reference)))

(event EventTick
  (params (DeltaSeconds :type Float%20%28single-precision%29))
  (bind _triggermesh (Variables|Default|GetTriggerMesh))
  (bind _interactref (Variables|Default|GetInteractRef))
  (if (Variables|Default|GetInsideTriggerArea)
    (Utilities|IsValid _interactref
      (:Is%20Valid
        (if (Variables|/Game/Characters/Blueprints/BP_Player_Interact_Component.BP_Player_Interact_Component_C|GetInteract _interactref)
          (Utilities|FlowControl|DoOnce false :!label _label
            (:Completed
              (for _array_element (Variables|Traps|GetTraps)
                (BehaviorTree|ArmTrap _array_element))
              (Effects|SpawnEmitteratLocation "/Game/Art/Particles/AdvancedMagicFX13/Particles/P_ky_flash1.P_ky_flash1" (Transformation|GetWorldLocation _triggermesh) (Transformation|GetWorldRotation _triggermesh))
              (Audio|PlaySoundatLocation "/Game/Audio/bling_no.bling_no" (Transformation|GetWorldLocation (Variables|Default|GetDefaultSceneRoot)) "0, 0, 0" 1.0 1.0 0.0 0 0 0)))
          (else
            (goto _label Reset)))))))

(fn ConstructionScript)

(fn ArmTrap
  (params (Trap :type BP%20Base%20Trap%20Object%20Reference))
  (bind _returnvalue (AI|GetBlackboard Trap))
  (bind _trapstate (LocalVariables|GetTrapState))
  (bind _returnvalue_2 (Class|BlackboardComponent|GetValueasEnum _returnvalue _trapstate))
  (bind _returnvalue_3 (Utilities|Enum|ByteToEnumE_CurrentTrapState _returnvalue_2))
  (if (or (Utilities|Enum|Equal(Enum) _returnvalue_3 "NewEnumerator16") (Utilities|Enum|Equal(Enum) _returnvalue_3 "NewEnumerator18"))
    (AI|Components|Blackboard|SetValueasEnum _returnvalue (LocalVariables|GetTrapState) (LocalVariables|GetTimeBeforeArmed))
    (return)
    (else
      (return))))