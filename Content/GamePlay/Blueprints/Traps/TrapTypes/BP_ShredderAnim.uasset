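; Animated shredder trap prop that spins two shredder components in opposing pitch directions.
; On BeginPlay it starts a rotation timeline that drives both components on each update, using none of its track values.
; Each update adds the component's current relative rotation, with pitch nudged down or up, as a local delta, so rotation feeds back on itself rather than stepping by a constant amount.
; It contains no overlap or damage logic.
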(event EventBeginPlay
  (bind _shredder1 (Variables|Default|GetShredder1))
  (bind _shredder2 (Variables|Default|GetShredder2))
  (bind _relativerotation (Variables|/Script/Engine.SceneComponent|GetRelativeRotation _shredder1))
  (bind _relativerotation_2 (Variables|/Script/Engine.SceneComponent|GetRelativeRotation _shredder2))
  (Timeline|TimeLineRotation Play
    (:Update
      (Utilities|FlowControl|Sequence
        (:then_0
          (Transformation|AddLocalRotation (Variables|Default|GetShredder1) (Math|Rotator|MakeRotator (.roll _relativerotation) (- (.pitch _relativerotation) 0.1) (.yaw _relativerotation)) false false))
        (:then_1
          (Transformation|AddLocalRotation (Variables|Default|GetShredder2) (Math|Rotator|MakeRotator (.roll _relativerotation_2) (+ (.pitch _relativerotation_2) 0.1) (.yaw _relativerotation_2)) false false))))))

(event Collision|EventActorBeginOverlap
  (params (OtherActor :type Actor%20Object%20Reference)))

(event EventTick
  (params (DeltaSeconds :type Float%20%28single-precision%29)))

(fn ConstructionScript)