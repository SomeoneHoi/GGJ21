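; Bear trap Blueprint, a child of a trap base class that supplies the overlap and damage logic.
; It overrides DealDamage to call the parent, then plays a one-shot animation on the Beartrap mesh when damage succeeds, passing the parent's damaged and armed results through.
; Overlap and construction only forward to the parent, and a DisableTrapCompletely call is left unconnected, so it never runs.
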(event EventBeginPlay
  (|CallParentFunction) ; This node is disabled and will not be called.\nDrag off pins to build functionality.
)

(event Collision|EventActorBeginOverlap
  (params (OtherActor :type Actor%20Object%20Reference))
  (|CallParentFunction OtherActor))

(event EventTick
  (params (DeltaSeconds :type Float%20%28single-precision%29))
  (|CallParentFunction DeltaSeconds) ; This node is disabled and will not be called.\nDrag off pins to build functionality.
)

(fn ConstructionScript
  (|CallParentFunction))

(fn DealDamage
  (params (HitResult :type Hit%20Result%20Structure))
  (bind (_trapdamagedsuccesfully _traparmed) (|CallParentFunction HitResult))
  (if _trapdamagedsuccesfully
    (Components|Animation|PlayAnimation (Variables|Default|GetBeartrap) "/Game/Art/Models/BearTrapAnimated_Anim.BearTrapAnimated_Anim" false)
    (return _trapdamagedsuccesfully _traparmed)))