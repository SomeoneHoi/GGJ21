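; BP_Trap_BBQ is a fire trap that damages AI characters, built as a child of a parent trap class.
; Arming spawns a fire particle emitter at the damage overlap shape, then runs the parent arm logic.
; Tick rebinds the damage event every frame, and that handler calls Hit on AI characters with a fixed enum value.
; Triggering simply defers to the parent.
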(event Custom|DamageActor
  (params (Actor :type Actor%20Soft%20Object%20Reference))
  (bind _asbp_aicharacters (Utilities|Casting|CastToBP_AICharacters (Utilities|ResolveSoftReference Actor)))
  (Default|Hit _asbp_aicharacters "NewEnumerator0"))

(event EventBeginPlay
  (|CallParentFunction) ; This node is disabled and will not be called.\nDrag off pins to build functionality.
)

(event Collision|EventActorBeginOverlap
  (params (OtherActor :type Actor%20Object%20Reference))
  (|CallParentFunction OtherActor) ; This node is disabled and will not be called.\nDrag off pins to build functionality.
)

(event EventTick
  (params (DeltaSeconds :type Float%20%28single-precision%29))
  (|CallParentFunction DeltaSeconds)
  (EventDispatchers|BindEventtoDamage (delegate Custom|DamageActor)))

(fn ConstructionScript
  (|CallParentFunction))

(fn TriggerTrap
  (bind _traptriggeredsuccesfully (|CallParentFunction))
  (return _traptriggeredsuccesfully))

(fn ArmTrap
  (bind _damageoverlapshape (Variables|Default|GetDamageOverlapShape))
  (Effects|SpawnEmitteratLocation "/Game/Art/Particles/P_Fire.P_Fire" (Transformation|GetWorldLocation _damageoverlapshape) (Transformation|GetWorldRotation _damageoverlapshape))
  (|CallParentFunction))