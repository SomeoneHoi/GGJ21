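; BP_TrapLever is a lever actor that arms every trap in its Traps list when the player interacts inside its trigger area.
; BeginPlay caches the interact component from BP_Player, printing a warning if it is missing.
; Trigger overlaps track the player's presence and print debug messages.
; Tick polls the component's Interact flag while the player is inside, clearing it before calling ArmTrap on each trap.
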(event OnComponentBeginOverlap(TriggerArea)
  (params (OverlappedComponent :type Primitive%20Component%20Object%20Reference) (OtherActor :type Actor%20Object%20Reference) (OtherComp :type Primitive%20Component%20Object%20Reference) (OtherBodyIndex :type Integer) (bFromSweep :type Boolean) (SweepResult :type Hit%20Result%20Structure%20%28by%20ref%29))
  (Utilities|Casting|CastToBP_Player OtherActor)
  (Variables|Default|SetInsideTriggerArea true)
  (Development|PrintString (Utilities|String|Append (Utilities|GetDisplayName self) "Lever area entered")))

(event OnComponentEndOverlap(TriggerArea)
  (params (OverlappedComponent :type Primitive%20Component%20Object%20Reference) (OtherActor :type Actor%20Object%20Reference) (OtherComp :type Primitive%20Component%20Object%20Reference) (OtherBodyIndex :type Integer))
  (Utilities|Casting|CastToBP_Player OtherActor)
  (Variables|Default|SetInsideTriggerArea false)
  (Development|PrintString (Utilities|String|Append (Utilities|GetDisplayName self) "Lever area left")))

(event EventBeginPlay
  (bind _returnvalue (Actor|GetActorOfClass "/Game/Characters/Blueprints/BP_Player.BP_Player_C"))
  (Utilities|IsValid (Actor|GetComponentbyClass _returnvalue "/Game/Characters/Blueprints/BP_Player_Interact_Component.BP_Player_Interact_Component_C")
    (:Is%20Valid
      (Variables|Default|SetInteractRef (Actor|GetComponentbyClass _returnvalue "/Game/Characters/Blueprints/BP_Player_Interact_Component.BP_Player_Interact_Component_C")))
    (:Is%20Not%20Valid
      (Development|PrintString "Warning: BP_Player does not have an BP_Interact_Component required for use in BP_TrapTrigger" true true "(R=1.000000,G=0.000000,B=0.000000,A=1.000000)" 1e+01))))

(event Collision|EventActorBeginOverlap
  (params (OtherActor :type Actor%20Object%20Reference)))

(event EventTick
  (params (DeltaSeconds :type Float%20%28single-precision%29))
  (bind _interactref (Variables|Default|GetInteractRef))
  (if (Variables|Default|GetInsideTriggerArea)
    (Utilities|IsValid _interactref
      (:Is%20Valid
        (if (Variables|/Game/Characters/Blueprints/BP_Player_Interact_Component.BP_Player_Interact_Component_C|GetInteract _interactref)
          (Variables|/Game/Characters/Blueprints/BP_Player_Interact_Component.BP_Player_Interact_Component_C|SetInteract _interactref false)
          (for _array_element (Variables|Traps|GetTraps)
            (Default|ArmTrap _array_element)))))))

(fn ConstructionScript)