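; Player component that turns forward and right input from the PC_InGame controller into walking movement for its owning character.
; On BeginPlay it casts the owner's controller to PC_InGame and binds to its move-forward and move-right events, stopping if the cast fails.
; Each handler feeds AddMovementInput along the control rotation's yaw only, so movement stays on the horizontal plane regardless of camera pitch or roll.
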(event Custom|DelegateMoveForward
  (params (Value :type Float%20%28single-precision%29))
  (CallFunction|MoveForward Value))

(event Custom|DelegateMoveRight
  (params (Value :type Float%20%28single-precision%29))
  (CallFunction|MoveRight Value))

(event EventBeginPlay
  (|CallParentFunction)
  (bind _aspc_in_game (Utilities|Casting|CastToPC_InGame (Pawn|GetController (Variables|Default|GetOwner))))
  (EventDispatchers|BindEventtoOnMoveForward _aspc_in_game (delegate Custom|DelegateMoveForward))
  (EventDispatchers|BindEventtoOnMoveRight _aspc_in_game (delegate Custom|DelegateMoveRight)))

(event EventTick
  (params (DeltaSeconds :type Float%20%28single-precision%29))
  (|CallParentFunction DeltaSeconds) ; This node is disabled and will not be called.\nDrag off pins to build functionality.
)

(fn MoveForward
  (params (Value :type Float%20%28single-precision%29))
  (Pawn|Input|AddMovementInput (Variables|Default|GetOwner) (Math|Vector|GetForwardVector (Math|Rotator|MakeRotator 0.0 0.0 (.Yaw (Math|Rotator|BreakRotator (Pawn|GetControlRotation (Variables|Default|GetOwner) :!class /Script/Engine.Pawn))))) Value false))

(fn MoveRight
  (params (Value :type Float%20%28single-precision%29))
  (Pawn|Input|AddMovementInput (Variables|Default|GetOwner) (Math|Vector|GetRightVector (Math|Rotator|MakeRotator 0.0 0.0 (.Yaw (Math|Rotator|BreakRotator (Pawn|GetControlRotation (Variables|Default|GetOwner) :!class /Script/Engine.Pawn))))) Value false))