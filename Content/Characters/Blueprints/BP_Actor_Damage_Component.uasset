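; Damage component that gives its owning Pawn health, starting from an initial value on BeginPlay.
; It binds to the owner's any-damage event, prints debug details and subtracts the damage from current health.
; Shredder trap hits spawn a delayed fluff emitter on player 0's mesh, whoever the owner is.
; At zero health, a Character owner ragdolls through mesh physics and has movement disabled.
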(event Custom|Spawn%20Emitter
  (if (== (Utilities|GetClass (stale Custom|DelegateOnTakeAnyDamage DamageCauser)) "/Game/GamePlay/Blueprints/BP_Trap_Shredder.BP_Trap_Shredder_C")
    (Utilities|FlowControl|Delay 0.5)
    (bind _asbp_player (Utilities|Casting|CastToBP_Player (Game|GetPlayerCharacter 0)))
    (Effects|SpawnEmitterAttached "/Game/Art/Particles/P_Fluff.P_Fluff" (Variables|/Script/Engine.Character|GetMesh _asbp_player) "None" (Transformation|GetWorldLocation (Variables|/Script/Engine.Character|GetMesh _asbp_player)) (Transformation|GetWorldRotation (Variables|/Script/Engine.Character|GetMesh _asbp_player)))))

(event Custom|DelegateOnTakeAnyDamage
  (params (DamagedActor :type Actor%20Object%20Reference) (Damage :type Float%20%28single-precision%29) (DamageType :type Damage%20Type%20Object%20Reference) (InstigatedBy :type Controller%20Object%20Reference) (DamageCauser :type Actor%20Object%20Reference))
  (CallFunction|SpawnEmitter)
  (Development|PrintString (Utilities|String|Append "Damage:" (Utilities|String|ToString(Float) Damage) "Damage type:" (Utilities|GetDisplayName DamageType) "Damage Causer:" (Utilities|GetDisplayName DamageCauser)) true true "(R=0.000000,G=0.660000,B=1.000000,A=1.000000)" 1e+01)
  (bind _output_get (Variables|Default|SetCurrentHealth (- (Variables|Default|GetCurrentHealth) Damage)))
  (if (<= _output_get 0.0)
    (CallFunction|Dying)
    (Utilities|FlowControl|Delay 0.2)))

(event EventBeginPlay
  (bind _aspawn (Utilities|Casting|CastToPawn (Components|GetOwner)))
  (EventDispatchers|BindEventtoOnTakeAnyDamage _aspawn (delegate Custom|DelegateOnTakeAnyDamage))
  (Variables|Default|SetCurrentHealth (Variables|Default|GetInitialHealth)))

(event EventTick
  (params (DeltaSeconds :type Float%20%28single-precision%29)))

(fn Dying
  (bind _ascharacter (Utilities|Casting|CastToCharacter (Components|GetOwner))
    (:then
      (Physics|SetSimulatePhysics (Variables|/Script/Engine.Character|GetMesh _ascharacter) true)
      (Pawn|Components|CharacterMovement|DisableMovement (Variables|/Script/Engine.Character|GetCharacterMovement _ascharacter))
      (return))
    (:CastFailed
      (return))))