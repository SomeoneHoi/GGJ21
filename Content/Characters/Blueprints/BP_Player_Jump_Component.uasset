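; BP_Player_Jump_Component is a player component that makes its owning character jump in response to controller input.
; On BeginPlay it casts the owner's controller to PC_InGame and binds DelegateJump to that controller's OnJump event.
; The delegate's boolean selects between Jump and StopJumping on the owner, so the component itself reads no input and runs no Tick logic.
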(event Custom|DelegateJump
  (params (bool :type Boolean))
  (bind _owner (Variables|Default|GetOwner))
  (if bool
    (Character|Jump _owner)
    (else
      (Character|StopJumping _owner))))

(event EventBeginPlay
  (|CallParentFunction)
  (bind _aspc_in_game (Utilities|Casting|CastToPC_InGame (Pawn|GetController (Variables|Default|GetOwner))))
  (EventDispatchers|BindEventtoOnJump _aspc_in_game (delegate Custom|DelegateJump)))

(event EventTick
  (params (DeltaSeconds :type Float%20%28single-precision%29))
  (|CallParentFunction DeltaSeconds) ; This node is disabled and will not be called.\nDrag off pins to build functionality.
)