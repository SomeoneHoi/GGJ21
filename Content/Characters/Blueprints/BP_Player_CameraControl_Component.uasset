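; Player component that drives camera look by applying yaw and pitch input to the owning character.
; On BeginPlay it binds to the turn and look-up events of the in-game player controller, stopping if the controller is not PC_InGame.
; Absolute axis values pass straight through, while rate-based values are scaled by base rates and world delta seconds for frame-rate independence.
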(event Custom|DelegateTurn
  (params (Value :type Float%20%28single-precision%29))
  (CallFunction|Turn Value))

(event Custom|DelegateLookUp
  (params (Value :type Float%20%28single-precision%29))
  (CallFunction|LookUp Value))

(event Custom|DelegateTurnRate
  (params (Value :type Float%20%28single-precision%29))
  (CallFunction|Turn (* Value (Variables|Default|GetBaseRate) (Utilities|Time|GetWorldDeltaSeconds))))

(event Custom|DelegateLookUpRate
  (params (Value :type Float%20%28single-precision%29))
  (CallFunction|LookUp (* Value (Variables|Default|GetBaseLookUpRate) (Utilities|Time|GetWorldDeltaSeconds))))

(event EventBeginPlay
  (|CallParentFunction)
  (bind _aspc_in_game (Utilities|Casting|CastToPC_InGame (Pawn|GetController (Variables|Default|GetOwner))))
  (EventDispatchers|BindEventtoOnTurn _aspc_in_game (delegate Custom|DelegateTurn))
  (EventDispatchers|BindEventtoOnTurnRate _aspc_in_game (delegate Custom|DelegateTurnRate))
  (EventDispatchers|BindEventtoOnLookUp _aspc_in_game (delegate Custom|DelegateLookUp))
  (EventDispatchers|BindEventtoOnLookUpRate _aspc_in_game (delegate Custom|DelegateLookUpRate)))

(event EventTick
  (params (DeltaSeconds :type Float%20%28single-precision%29)))

(fn Turn
  (params (Value :type Float%20%28single-precision%29))
  (Pawn|Input|AddControllerYawInput (Variables|Default|GetOwner) Value))

(fn LookUp
  (params (Value :type Float%20%28single-precision%29))
  (Pawn|Input|AddControllerPitchInput (Variables|Default|GetOwner) Value))