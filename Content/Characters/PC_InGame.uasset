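; PC_InGame is the in-game input relay, by its name a player controller, that turns player input into event dispatcher calls.
; Look, turn and movement axes pass their values straight through to matching OnX dispatchers.
; Jump and Interact broadcast true on press and false on release, with no gameplay logic handled here.
; An unconnected AI MoveTo node, noted for moving to actor AI teddies, never runs.
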(event EventBeginPlay)

(event EventTick
  (params (DeltaSeconds :type Float%20%28single-precision%29)))

(event Input|ActionEvents|InputActionJump
  (params (Key :type Key%20Structure :default "None"))
  (:Pressed
    (Default|CallOnJump true))
  (:Released
    (Default|CallOnJump false)))

(event Input|ActionEvents|InputActionInteract
  (params (Key :type Key%20Structure :default "None"))
  (:Pressed
    (Default|CallOnInteract true))
  (:Released
    (Default|CallOnInteract false)))

(event Input|AxisEvents|InputAxisTurn
  (params (AxisValue :type Float%20%28single-precision%29))
  (Default|CallOnTurn AxisValue))

(event Input|AxisEvents|InputAxisLookUp
  (params (AxisValue :type Float%20%28single-precision%29))
  (Default|CallOnLookUp AxisValue))

(event Input|AxisEvents|InputAxisTurnRate
  (params (AxisValue :type Float%20%28single-precision%29))
  (Default|CallOnTurnRate AxisValue))

(event Input|AxisEvents|InputAxisLookUpRate
  (params (AxisValue :type Float%20%28single-precision%29))
  (Default|CallOnLookUpRate AxisValue))

(event Input|AxisEvents|InputAxisMoveForward
  (params (AxisValue :type Float%20%28single-precision%29))
  (Default|CallOnMoveForward AxisValue))

(event Input|AxisEvents|InputAxisMoveRight
  (params (AxisValue :type Float%20%28single-precision%29))
  (Default|CallOnMoveRight AxisValue))

(fn ConstructionScript)