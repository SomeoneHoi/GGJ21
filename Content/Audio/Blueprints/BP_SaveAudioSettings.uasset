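; BP_SaveAudioSettings is a save game object that stores audio volume per sound channel in a SoundSettings map.
; SetAudioChannel adds or overwrites a single channel's volume, while SetAudioSettings replaces the whole map.
; SaveAudioSettings writes the object itself to the slot named by SaveAudioSettingsName and returns the save result.
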(fn SaveAudioSettings
  (bind _returnvalue (SaveGame|SaveGametoSlot self (Variables|Default|GetSaveAudioSettingsName)))
  (return _returnvalue))

(fn SetAudioChannel
  (params (SoundChannel :type E_SoundChannels%20Enum :default "NewEnumerator0") (SoundVolume :type Float%20%28single-precision%29))
  (Utilities|Map|Add (Variables|Default|GetSoundSettings) SoundChannel SoundVolume)
  (return))

(fn SetAudioSettings
  (params (SoundChannels :type Map%20of%20E_SoundChannels%20Enums%20to%20Float%20%28single-precision%29s :default "NewEnumerator0"))
  (Variables|Default|SetSoundSettings SoundChannels)
  (return))